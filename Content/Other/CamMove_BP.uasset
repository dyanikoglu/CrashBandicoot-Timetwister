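; Camera-turn trigger volume that rotates the player's view yaw while CrashBandicootPlayerBP is inside MoveCam and returns it to InterpBase on exit.
; The construction script picks the target yaw, InterpTo, from the TurnSide setting (Left or Right).
; Each overlap event starts a fast looping timer that eases control rotation with RInterpTo, pauses the opposite timer, and snaps yaw once nearly equal to the target.
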(event `self.MoveCam.OnComponentBeginOverlap`
  (params (OverlappedComponent :type "PrimitiveComponent Object Reference") (OtherActor :type "Actor Object Reference") (OtherComp :type "PrimitiveComponent Object Reference") (OtherBodyIndex :type Integer) (bFromSweep :type Boolean) (SweepResult :type "HitResult Structure (by ref)"))
  (cast `/Game/Main/Blueprints/CrashBandicootPlayerBP` OtherActor)
  (`KismetSystemLibrary.K2_PauseTimerHandle` (`self.INTERP2_PAUSE`))
  (bind _returnvalue (`KismetSystemLibrary.K2_SetTimerDelegate` (delegate `InterpEvent1`) 0.001 true))
  (set `self.INTERP1_PAUSE` _returnvalue))

(event `InterpEvent1`
  (bind _returnvalue (`GameplayStatics.GetPlayerCharacter` 0))
  (bind _returnvalue_2 (`Pawn.GetControlRotation` _returnvalue))
  (bind (_returnvalue_roll _returnvalue_pitch _returnvalue_yaw) (`KismetMathLibrary.BreakRotator` (`Pawn.GetControlRotation` (`GameplayStatics.GetPlayerCharacter` 0))))
  (`KismetSystemLibrary.K2_PauseTimerHandle` (`self.INTERP2_PAUSE`))
  (`Controller.SetControlRotation` (`Pawn.GetController` _returnvalue) (`KismetMathLibrary.RInterpTo` _returnvalue_2 (`KismetMathLibrary.MakeRotator` (.roll _returnvalue_2) (.pitch _returnvalue_2) (`self.interpTo`)) (`GameplayStatics.GetWorldDeltaSeconds`) 0.5))
  (if (`KismetMathLibrary.NearlyEqual_FloatFloat` _returnvalue_yaw (`self.interpTo`) 0.5)
    (`KismetSystemLibrary.K2_PauseTimerHandle` (`self.INTERP1_PAUSE`))
    (`Controller.SetControlRotation` (`Pawn.GetController` (`GameplayStatics.GetPlayerCharacter` 0)) (`KismetMathLibrary.MakeRotator` _returnvalue_roll _returnvalue_pitch (`self.interpTo`)))))

(event `self.MoveCam.OnComponentEndOverlap`
  (params (OverlappedComponent :type "PrimitiveComponent Object Reference") (OtherActor :type "Actor Object Reference") (OtherComp :type "PrimitiveComponent Object Reference") (OtherBodyIndex :type Integer))
  (cast `/Game/Main/Blueprints/CrashBandicootPlayerBP` OtherActor)
  (`KismetSystemLibrary.K2_PauseTimerHandle` (`self.INTERP1_PAUSE`))
  (bind _returnvalue (`KismetSystemLibrary.K2_SetTimerDelegate` (delegate `InterpEvent2`) 0.001 true))
  (set `self.INTERP2_PAUSE` _returnvalue))

(event `InterpEvent2`
  (bind _returnvalue (`GameplayStatics.GetPlayerCharacter` 0))
  (bind (_returnvalue_roll _returnvalue_pitch _returnvalue_yaw) (`KismetMathLibrary.BreakRotator` (`Pawn.GetControlRotation` (`GameplayStatics.GetPlayerCharacter` 0))))
  (bind _returnvalue_2 (`Pawn.GetControlRotation` _returnvalue))
  (`KismetSystemLibrary.K2_PauseTimerHandle` (`self.INTERP1_PAUSE`))
  (`Controller.SetControlRotation` (`Pawn.GetController` _returnvalue) (`KismetMathLibrary.RInterpTo` _returnvalue_2 (`KismetMathLibrary.MakeRotator` (.roll _returnvalue_2) (.pitch _returnvalue_2) (`self.interpBase`)) (`GameplayStatics.GetWorldDeltaSeconds`) 0.5))
  (if (`KismetMathLibrary.NearlyEqual_FloatFloat` _returnvalue_yaw (`self.interpBase`) 0.5)
    (`KismetSystemLibrary.K2_PauseTimerHandle` (`self.INTERP2_PAUSE`))
    (`Controller.SetControlRotation` (`Pawn.GetController` (`GameplayStatics.GetPlayerCharacter` 0)) (`KismetMathLibrary.MakeRotator` _returnvalue_roll _returnvalue_pitch (`self.interpBase`)))))

(fn `UserConstructionScript`
  (switch `/Game/Other/CamMove_Enum` (`self.Turn Side`)
    (:`NewEnumerator0`
      (set `self.interpTo` 230.0))
    (:`NewEnumerator1`
      (set `self.interpTo` -55.0))))