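; Crash's Wumpa rocket launcher, toggled by Activate and Deactivate, which show or hide the launcher and its laser sight.
; While active, Tick line-traces forward to place the laser beam, calls aim-update dispatchers, and beeps once on acquiring an enemy or eligible crate.
; Fire spawns a Wumpa_Projectile with smoke, sound, camera shake and recoil on launcher and player mesh, using a delayed DoOnce reset as cooldown.
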(event `Activate`
  (`SceneComponent.SetHiddenInGame` (`self.rocketlauncher`) false false)
  (`SceneComponent.SetHiddenInGame` (`self.LaserParticle`) false false)
  (`ActorComponent.Activate` (`self.LaserParticle`) false)
  (set `self.isActive?` true)
  (`ActorComponent.Activate` (`self.rocket_idle`) false))

(event `Deactivate`
  (`self.hideAim`)
  (`SceneComponent.SetHiddenInGame` (`self.rocketlauncher`) true false)
  (`SceneComponent.SetHiddenInGame` (`self.LaserParticle`) true false)
  (`ActorComponent.Deactivate` (`self.LaserParticle`))
  (set `self.isActive?` false)
  (`ActorComponent.Deactivate` (`self.rocket_idle`)))

(event `self.ReceiveTick`
  (params (DeltaSeconds :type "Float (single-precision)"))
  (bind _lasersource (`self.LaserSource`))
  (bind _laserparticle (`self.LaserParticle`))
  (bind _returnvalue (`SceneComponent.K2_GetComponentLocation` _lasersource))
  (bind _returnvalue_2 (+ _returnvalue (* (`SceneComponent.GetForwardVector` _lasersource) 5000.0)))
  (if (`self.isActive?`)
    (bind (_outhit _returnvalue_3) (`KismetSystemLibrary.LineTraceSingle` _returnvalue _returnvalue_2 "TraceTypeQuery1"))
    (if _returnvalue_3
      (set `self.screen` (`.TraceEnd` (`GameplayStatics.BreakHitResult` _outhit)))
      (set `self.LaserTargetLoc` (`.Location` (`GameplayStatics.BreakHitResult` _outhit)))
      (else
        (set `self.LaserTargetLoc` _returnvalue_2)))
    (`ParticleSystemComponent.SetBeamSourcePoint` _laserparticle 0 _returnvalue 0)
    (`ParticleSystemComponent.SetBeamTargetPoint` _laserparticle 0 (`self.LaserTargetLoc`) 0)
    (cast `/Game/Models/Enemy/Enemy_Parent` (`.HitActor` (`GameplayStatics.BreakHitResult` _outhit))
      (:`then`
        (if (not (`self.isOnEnemy?`)) :!label _label
          (`GameplayStatics.PlaySoundAtLocation` "/Game/Sounds/launcher_beep.launcher_beep" (0.0 0.0 0.0) (struct) 1.0 1.0 0.0 null null null)
          (set `self.isOnEnemy?` true)))
      (:`CastFailed`
        (bind _ascrate (cast `/Game/Models/General/Crate/Crate` (`.HitActor` (`GameplayStatics.BreakHitResult` _outhit)))
          (:`then`
            (bind _cratetype (`/Game/Models/General/Crate/Crate.CrateType` _ascrate))
            (if (or (`|EnumEquality` _cratetype "NewEnumerator7") (`|EnumEquality` _cratetype "NewEnumerator8"))
              _
              (else
                (goto _label))))
          (:`CastFailed`
            (if (`self.isOnEnemy?`)
              (set `self.isOnEnemy?` false))))))
    (`self.updateAim`)
    (goto _label_2 :!via `Reset`)
    (else
      (`/Engine/EditorBlueprintResources/StandardMacros.DoOnce` false :!label _label_2
        (:`Completed`
          (`self.hideAim`))))))

(event `Fire`
  (bind _rocketlauncher (`self.rocketlauncher`))
  (bind _launchlocation (`self.LaunchLocation`))
  (bind _rocketlauncher_2 (`self.rocketlauncher`))
  (`/Engine/EditorBlueprintResources/StandardMacros.DoOnce` false :!label _label_3
    (:`Completed`
      (`GameplayStatics.SpawnEmitterAtLocation` null (`SceneComponent.K2_GetComponentLocation` (`self.SmokeSpawn`)))
      (`|SpawnActorFromClass` "/Game/Main/Crash/RocketLauncher/Wumpa_Projectile.Wumpa_Projectile_C" (`KismetMathLibrary.MakeTransform` (`SceneComponent.K2_GetComponentLocation` _launchlocation) (`SceneComponent.K2_GetComponentRotation` _launchlocation)) "Undefined" "OverrideRootScale" null null)
      (`PlayerController.ClientStartCameraShake` :`self` (`GameplayStatics.GetPlayerController` 0) :`Shake` "/Game/Main/Crash/RocketLauncher/shake.shake_C")
      (`GameplayStatics.PlaySoundAtLocation` "/Game/Sounds/rocket_hit.rocket_hit" (0.0 0.0 0.0) (struct) 1.0 1.0 0.0 null null null)
      (`SceneComponent.K2_SetRelativeLocation` _rocketlauncher (- (`SceneComponent.RelativeLocation` _rocketlauncher) (0.0 0.0 5.0)) false false)
      (`KismetSystemLibrary.Delay` 0.1)
      (`SceneComponent.K2_SetRelativeLocation` _rocketlauncher_2 (- (`SceneComponent.RelativeLocation` _rocketlauncher_2) (0.0 0.0 -5.0)) false false)
      (bind _ascrash_bandicoot_player_bp (cast `/Game/Main/Blueprints/CrashBandicootPlayerBP` (`GameplayStatics.GetPlayerCharacter` 0)))
      (bind _mesh (`Character.Mesh` _ascrash_bandicoot_player_bp))
      (bind _returnvalue (`SceneComponent.GetRelativeTransform` _mesh))
      (`SceneComponent.K2_SetRelativeRotation` _mesh (`KismetMathLibrary.MakeRotator` (+ (.roll (.rotation _returnvalue)) -2.0) (.pitch (.rotation _returnvalue)) (.yaw (.rotation _returnvalue))) false false)
      (`KismetSystemLibrary.Delay` 0.05)
      (bind _mesh_2 (`Character.Mesh` _ascrash_bandicoot_player_bp))
      (bind _returnvalue_2 (`SceneComponent.GetRelativeTransform` _mesh_2))
      (`SceneComponent.K2_SetRelativeRotation` _mesh_2 (`KismetMathLibrary.MakeRotator` (+ (.roll (.rotation _returnvalue_2)) 2.0) (.pitch (.rotation _returnvalue_2)) (.yaw (.rotation _returnvalue_2))) false false)
      (`KismetSystemLibrary.Delay` 0.4)
      (goto _label_3 :!via `Reset`))))

(fn `CreateBeam`
  (params (StartLocation :type "Vector Structure") (EndLocation :type "Vector Structure")))

(fn `UserConstructionScript`)