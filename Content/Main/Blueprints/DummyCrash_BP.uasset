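; DummyCrash_BP is a dummy Crash actor that plays a deflating-balloon style effect, shrinking and darting around while a deflate sound plays.
; On BeginPlay it caches the start transform and starts two looping timers that drive VInterpTo on Crash2's location and scale.
; Each time location nears its target, a non-looping MultiGate picks the next hard-coded offset from the start, forming an erratic path that ends far away.
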(event `self.ReceiveBeginPlay`
  (set `self.SVInterpBase` (`SceneComponent.K2_GetComponentScale` (`self.crash2`)))
  (set `self.SVInterpTarget` (0.1 0.1 0.1))
  (set `self.VInterpBase` (`SceneComponent.K2_GetComponentLocation` (`self.crash2`)))
  (set `self.VInterpTarget` (+ (`self.VInterpBase`) (200.0 -250.0 100.0)))
  (`KismetSystemLibrary.K2_SetTimerDelegate` (delegate `InterpLocation`) 0.01 true)
  (`KismetSystemLibrary.K2_SetTimerDelegate` (delegate `Interp Scale`) 0.01 true)
  (`GameplayStatics.PlaySoundAtLocation` "/Game/Sounds/CrashGeneral/crash_deflat.crash_deflat"))

(event `InterpLocation`
  (bind _vinterptarget (`self.VInterpTarget`))
  (bind _returnvalue (`SceneComponent.K2_GetComponentLocation` (`self.crash2`)))
  (`SceneComponent.K2_SetWorldLocation` (`self.crash2`) (`KismetMathLibrary.VInterpTo` _returnvalue _vinterptarget 0.01 7.0) false false)
  (if (== _returnvalue _vinterptarget :`ErrorTolerance` 150.0)
    (`|MultiGate` false false 0
      (:`Out 0`
        (set `self.VInterpTarget` (+ (`self.VInterpBase`) (-300.0 20.0 -105.0))))
      (:`Out 1`
        (set `self.VInterpTarget` (+ (`self.VInterpBase`) (350.0 -150.0 50.0))))
      (:`Out 2`
        (set `self.VInterpTarget` (+ (`self.VInterpBase`) (-250.0 100.0 -75.0))))
      (:`Out 3`
        (set `self.VInterpTarget` (+ (`self.VInterpBase`) (300.0 -700.0 100.0))))
      (:`Out 4`
        (set `self.VInterpTarget` (+ (`self.VInterpBase`) (-300.0 150.0 -150.0))))
      (:`Out 5`
        (set `self.VInterpTarget` (+ (`self.VInterpBase`) (-400.0 -900.0 -50.0))))
      (:`Out 6`
        (set `self.VInterpTarget` (+ (`self.VInterpBase`) (500.0 50.0 250.0))))
      (:`Out 7`
        (set `self.VInterpTarget` (+ (`self.VInterpBase`) (400.0 -2500.0 500.0)))))))

(event `Interp Scale`
  (`SceneComponent.SetWorldScale3D` (`self.crash2`) (`KismetMathLibrary.VInterpTo` (`SceneComponent.K2_GetComponentScale` (`self.crash2`)) (`self.SVInterpTarget`) 0.01 1.5)))

(fn `UserConstructionScript`)