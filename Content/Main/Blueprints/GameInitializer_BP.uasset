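; Level initializer for a Crash Bandicoot game that handles checkpoint saves, player spawning and crate tracking.
; Construction script builds checkpoint spawn transforms and totals countable crates, using actor tags as array indices.
; Init loads the "save1" slot, removes previously broken crates and binds crate destruction events.
; Destroying a checkpoint crate saves checkpoint, broken crates, lives and Wumpa; Spawn places the player there and restores both stats.
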(event `Spawn`
  (bind _checkpoint (`self.checkPoint`))
  ;[1 1 1] Spawn
  (switch `int` _checkpoint
    (:`Default`
      (`|SpawnActorFromClass` "/Game/Main/Blueprints/CrashBandicootPlayerBP.CrashBandicootPlayerBP_C" (`|GetArrayItem` (`self.checkPointArr`) _checkpoint) "Undefined" "OverrideRootScale" null null)
      (bind _ascheckpoint_save (cast `/Game/Main/CheckpointSave` (`self.subClass`)))
      (bind _ascrash_bandicoot_player_bp (cast `/Game/Main/Blueprints/CrashBandicootPlayerBP` (`GameplayStatics.GetPlayerCharacter` 0)))
      (set `/Game/Main/Blueprints/CrashBandicootPlayerBP.Lives` (`/Game/Main/CheckpointSave.life` _ascheckpoint_save) _ascrash_bandicoot_player_bp)
      (set `/Game/Main/Blueprints/CrashBandicootPlayerBP.wumpaCount` (`/Game/Main/CheckpointSave.wumpaCount` _ascheckpoint_save) _ascrash_bandicoot_player_bp))))

(event `Save` :!signature `self.OnDestroyed`
  (params (DestroyedActor :type "Actor Object Reference"))
  ;[1 1 1] SAVE
  (`KismetArrayLibrary.Array_Set` (`self.tempDestroyedCrates`) (`KismetStringLibrary.Conv_StringToInt` (`KismetStringLibrary.Conv_NameToString` (`|GetArrayItem` (`Actor.Tags` DestroyedActor)))) true true)
  (bind _returnvalue (`GameplayStatics.DoesSaveGameExist` "save1"))
  (if _returnvalue
    (bind _returnvalue_2 (`GameplayStatics.LoadGameFromSlot` "save1"))
    (bind _output_get (set `self.subClass` _returnvalue_2))
    (bind _ascheckpoint_save (cast `/Game/Main/CheckpointSave` _output_get))
    (set `/Game/Main/CheckpointSave.checkPoint` (`KismetStringLibrary.Conv_StringToInt` (`KismetStringLibrary.Conv_NameToString` (`|GetArrayItem` (`Actor.Tags` DestroyedActor) 1))) _ascheckpoint_save)
    (set `/Game/Main/CheckpointSave.brokenCrates` (`self.tempDestroyedCrates`) _ascheckpoint_save)
    (bind _ascrash_bandicoot_player_bp (cast `/Game/Main/Blueprints/CrashBandicootPlayerBP` (`GameplayStatics.GetPlayerCharacter` 0)))
    (set `/Game/Main/CheckpointSave.wumpaCount` (`/Game/Main/Blueprints/CrashBandicootPlayerBP.wumpaCount` _ascrash_bandicoot_player_bp) _ascheckpoint_save)
    (set `/Game/Main/CheckpointSave.life` (`/Game/Main/Blueprints/CrashBandicootPlayerBP.Lives` _ascrash_bandicoot_player_bp) _ascheckpoint_save)
    (`GameplayStatics.SaveGameToSlot` (`self.subClass`) "save1")))

(event `Init`
  ;[1 1 1] Init Section
  (`self.Load`)
  (bind _outactors (`GameplayStatics.GetAllActorsOfClass` "/Game/Models/General/Crate/Crate.Crate_C"))
  (for _array_element _outactors
    (if (`|EnumEquality` (`/Game/Models/General/Crate/Crate.CrateType` _array_element) "NewEnumerator11")
      (add `self.OnDestroyed` _array_element (delegate `Save`))))
  (bind _outactors_2 (`GameplayStatics.GetAllActorsOfClass` "/Game/Models/General/Crate/Crate.Crate_C"))
  (for _array_element_2 _outactors_2
    (bind _cratetype (`/Game/Models/General/Crate/Crate.CrateType` _array_element_2))
    (if (and (`|EnumInequality` _cratetype "NewEnumerator6") (`|EnumInequality` _cratetype "NewEnumerator8") (not (`/Game/Models/General/Crate/Crate.secretMETAL` _array_element_2)) (`|EnumInequality` _cratetype "NewEnumerator9") (`|EnumInequality` _cratetype "NewEnumerator11"))
      (add `self.OnDestroyed` _array_element_2 (delegate `AddTempDestroyedCrate`))
      (`KismetArrayLibrary.Array_Set` (`self.tempDestroyedCrates`) (`KismetStringLibrary.Conv_StringToInt` (`KismetStringLibrary.Conv_NameToString` (`|GetArrayItem` (`Actor.Tags` _array_element_2)))) false true))))

(event `AddTempDestroyedCrate` :!signature `self.OnDestroyed`
  (params (DestroyedActor :type "Actor Object Reference"))
  ;[1 1 1] Add Destroyed Crate
  (`KismetArrayLibrary.Array_Set` (`self.tempDestroyedCrates`) (`KismetStringLibrary.Conv_StringToInt` (`KismetStringLibrary.Conv_NameToString` (`|GetArrayItem` (`Actor.Tags` DestroyedActor)))) true true)
  (`/Engine/EditorBlueprintResources/StandardMacros.IncrementInt` (`self.destroyedCrates`)))

(event `Load`
  ;[1 1 1] LOAD
  (bind _returnvalue (`GameplayStatics.DoesSaveGameExist` "save1"))
  (if _returnvalue
    (bind _returnvalue_2 (`GameplayStatics.LoadGameFromSlot` "save1"))
    (bind _output_get (set `self.subClass` _returnvalue_2))
    (bind _ascheckpoint_save (cast `/Game/Main/CheckpointSave` _output_get))
    (set `self.checkPoint` (`/Game/Main/CheckpointSave.checkPoint` _ascheckpoint_save))
    (bind _outactors (`GameplayStatics.GetAllActorsOfClass` "/Game/Models/General/Crate/Crate.Crate_C"))
    (for _array_element _outactors
      (bind _brokencrates (`/Game/Main/CheckpointSave.brokenCrates` _ascheckpoint_save))
      (if (`|GetArrayItem` _brokencrates (`KismetStringLibrary.Conv_StringToInt` (`KismetStringLibrary.Conv_NameToString` (`|GetArrayItem` (`Actor.Tags` _array_element)))))
        (`self.K2_DestroyActor` _array_element)
        (`/Engine/EditorBlueprintResources/StandardMacros.IncrementInt` (`self.destroyedCrates`))))
    (set `self.tempDestroyedCrates` _brokencrates)
    (else
      (bind _returnvalue_3 (`GameplayStatics.CreateSaveGameObject` "/Game/Main/CheckpointSave.CheckpointSave_C"))
      (`GameplayStatics.SaveGameToSlot` _returnvalue_3 "save1")
      (set `self.checkPoint` 0))))

(fn `UserConstructionScript`
  (bind _outactors (`GameplayStatics.GetAllActorsOfClass` "/Game/Models/General/Crate/Crate.Crate_C"))
  (for _array_element _outactors
    (if (`|EnumEquality` (`/Game/Models/General/Crate/Crate.CrateType` _array_element) "NewEnumerator11")
      (`KismetArrayLibrary.Array_Set` (`self.checkPointArr`) (`KismetStringLibrary.Conv_StringToInt` (`KismetStringLibrary.Conv_NameToString` (`|GetArrayItem` (`Actor.Tags` _array_element) 1))) (`KismetMathLibrary.MakeTransform` (+ (`SceneComponent.K2_GetComponentLocation` (`/Game/Models/General/Crate/Crate.Spawn` _array_element)) (0.0 0.0 100.0)) (struct :`Yaw` -90.0)) true)))
  (bind _outactors_2 (`GameplayStatics.GetAllActorsOfClass` "/Game/Models/General/Crate/Crate.Crate_C"))
  (for _array_element_2 _outactors_2
    (bind _cratetype (`/Game/Models/General/Crate/Crate.CrateType` _array_element_2))
    (if (and (`|EnumInequality` _cratetype "NewEnumerator6") (`|EnumInequality` _cratetype "NewEnumerator8") (not (`/Game/Models/General/Crate/Crate.secretMETAL` _array_element_2)) (`|EnumInequality` _cratetype "NewEnumerator9"))
      (`/Engine/EditorBlueprintResources/StandardMacros.IncrementInt` (`self.totalCrates`)))))