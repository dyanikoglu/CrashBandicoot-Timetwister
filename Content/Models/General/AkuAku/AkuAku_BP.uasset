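; Aku Aku mask companion for the Crash Bandicoot player, with hidden, two power tiers and a god mode.
; Transition events set the state enum and swap visibility, feather materials, particles and sounds as the mask gains or loses tiers.
; God mode snaps the mask to the player's mesh socket and enables capsule overlaps that kill enemies and destroy crates.
; After a 20-second delay it reattaches as a companion in the second tier.
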(event `HIDDENtoSTATE1`
  (`SceneComponent.SetHiddenInGame` (`self.AkuAku`) false false)
  (set `self.State` "NewEnumerator0")
  (`GameplayStatics.PlaySoundAtLocation` "/Game/Sounds/akuaku.akuaku" (0.0 0.0 0.0) (struct) 2.0))

(event `STATE1toSTATE2`
  (set `self.State` "NewEnumerator1")
  (bind _returnvalue (`GameplayStatics.SpawnEmitterAtLocation` "/Game/Effects/Effects/FX_Treasure/Loot/P_Loot_Pickup.P_Loot_Pickup" (`SceneComponent.K2_GetComponentLocation` (`self.AkuAku`))))
  (`SceneComponent.SetRelativeScale3D` _returnvalue (0.8 0.8 0.8))
  (bind _returnvalue_2 (`GameplayStatics.SpawnEmitterAttached` "/Game/Effects/Effects/FX_Treasure/Gold_Bag/P_GoldSparkle_Bag_Lo_2.P_GoldSparkle_Bag_Lo_2" (`self.AkuAku`) "particle"))
  (bind _output_get (set `self.State2ParticleRef` _returnvalue_2))
  (`SceneComponent.SetRelativeScale3D` _output_get (0.1 0.1 0.1))
  (for _index (range 1 4)
    (`PrimitiveComponent.SetMaterial` (`self.AkuAku`) _index "/Game/Models/General/AkuAku/Yellow_Feather2_Mat.Yellow_Feather2_Mat")
    (`GameplayStatics.PlaySoundAtLocation` "/Game/Sounds/akuaku.akuaku")))

(event `STATE2toGODMODE`
  (bind _akuaku (`self.AkuAku`))
  (set `self.State` "NewEnumerator2")
  (bind _returnvalue (`GameplayStatics.SpawnEmitterAttached` "/Game/Effects/Effects/FX_Treasure/Gold_Bag/P_DeadMans_Loot.P_DeadMans_Loot" (`self.AkuAku`)))
  (`SceneComponent.SetRelativeScale3D` _returnvalue (0.25 0.25 0.25))
  (`PrimitiveComponent.SetCollisionProfileName` (`self.Capsule`) "OverlapAll")
  (`GameplayStatics.PlaySoundAtLocation` "/Game/Sounds/AkuAkuOST.AkuAkuOST")
  (bind _ascrash_bandicoot_player_bp (cast `/Game/Main/Blueprints/CrashBandicootPlayerBP` (`GameplayStatics.GetPlayerCharacter` 0)))
  (`SceneComponent.K2_AttachToComponent` (`self.AkuAku`) (`Character.Mesh` _ascrash_bandicoot_player_bp) "AkuAkuPlug" "SnapToTarget" "SnapToTarget" "KeepWorld" true)
  (`SkeletalMeshComponent.SetAnimationMode` (`self.AkuAku`) "AnimationSingleNode")
  (`KismetSystemLibrary.Delay` 20.0)
  (set `self.State` "NewEnumerator1")
  (`SceneComponent.K2_AttachToComponent` _akuaku (`/Game/Main/Blueprints/CrashBandicootPlayerBP.AkuAku` _ascrash_bandicoot_player_bp) "None" "SnapToTarget" "KeepRelative" "KeepWorld" true)
  (`SceneComponent.K2_SetRelativeRotation` _akuaku (struct :`Yaw` -90.0) false false)
  (`SkeletalMeshComponent.SetAnimationMode` (`self.AkuAku`) "AnimationBlueprint")
  (`PrimitiveComponent.SetCollisionProfileName` (`self.Capsule`) "NoCollision")
  (`ActorComponent.K2_DestroyComponent` _returnvalue))

(event `STATE2toSTATE1`
  (bind _returnvalue (`SceneComponent.K2_GetComponentLocation` (`self.AkuAku`)))
  (`GameplayStatics.PlaySoundAtLocation` "/Game/Sounds/akuaku_lost_crash.akuaku_lost_crash" _returnvalue)
  (`GameplayStatics.PlaySoundAtLocation` "/Game/Sounds/akuaku_lost.akuaku_lost" _returnvalue)
  (`ActorComponent.K2_DestroyComponent` (`self.State2ParticleRef`))
  (set `self.State` "NewEnumerator0")
  (`PrimitiveComponent.SetMaterial` (`self.AkuAku`) 1 "/Game/Models/General/AkuAku/Orange_Feather2_Mat.Orange_Feather2_Mat")
  (`PrimitiveComponent.SetMaterial` (`self.AkuAku`) 2 "/Game/Models/General/AkuAku/Purple_Feather2_Mat.Purple_Feather2_Mat")
  (`PrimitiveComponent.SetMaterial` (`self.AkuAku`) 3 "/Game/Models/General/AkuAku/Red_Feather2_Mat.Red_Feather2_Mat")
  (for _ (range 4)
    (`GameplayStatics.SpawnEmitterAtLocation` "/Game/Models/General/AkuAku/P_Feathers_Yellow.P_Feathers_Yellow" (`SceneComponent.K2_GetComponentLocation` (`self.AkuAku`)))))

(event `STATE1toHIDDEN`
  (bind _returnvalue (`SceneComponent.K2_GetComponentLocation` (`self.AkuAku`)))
  (`GameplayStatics.PlaySoundAtLocation` "/Game/Sounds/akuaku_lost_crash.akuaku_lost_crash" _returnvalue)
  (`GameplayStatics.PlaySoundAtLocation` "/Game/Sounds/akuaku_lost.akuaku_lost" _returnvalue)
  (set `self.State` "NewEnumerator3")
  (`SceneComponent.SetHiddenInGame` (`self.AkuAku`) true false)
  (`GameplayStatics.SpawnEmitterAtLocation` "/Game/Models/General/AkuAku/P_Feathers_Orange.P_Feathers_Orange" (`SceneComponent.K2_GetComponentLocation` (`self.AkuAku`)))
  (`GameplayStatics.SpawnEmitterAtLocation` "/Game/Models/General/AkuAku/P_Feathers_Purple.P_Feathers_Purple" (`SceneComponent.K2_GetComponentLocation` (`self.AkuAku`)))
  (`GameplayStatics.SpawnEmitterAtLocation` "/Game/Models/General/AkuAku/P_Feathers_Red.P_Feathers_Red" (`SceneComponent.K2_GetComponentLocation` (`self.AkuAku`)))
  (`GameplayStatics.SpawnEmitterAtLocation` "/Game/Models/General/AkuAku/P_Feathers_Yellow.P_Feathers_Yellow" (`SceneComponent.K2_GetComponentLocation` (`self.AkuAku`))))

(event `self.Capsule.OnComponentBeginOverlap`
  (params (OverlappedComponent :type "PrimitiveComponent Object Reference") (OtherActor :type "Actor Object Reference") (OtherComp :type "PrimitiveComponent Object Reference") (OtherBodyIndex :type Integer) (bFromSweep :type Boolean) (SweepResult :type "HitResult Structure (by ref)"))
  (bind _asenemy_parent (cast `/Game/Models/Enemy/Enemy_Parent` OtherActor)
    (:`then`
      (set `/Game/Models/Enemy/Enemy_Parent.canDie?` true _asenemy_parent)
      (`/Game/Models/Enemy/Enemy_Parent.Standart Death` _asenemy_parent)
      (`/Engine/EditorBlueprintResources/StandardMacros.DoOnce` false :!label _label
        (:`Completed`
          (`GameplayStatics.SpawnSoundAtLocation` "/Game/Sounds/akuaku_hit.akuaku_hit")
          (goto _label :!via `Reset`))))
    (:`CastFailed`
      (bind _ascrate (cast `/Game/Models/General/Crate/Crate` OtherActor))
      (set `/Game/Models/General/Crate/Crate.directExplosion` true _ascrate)
      (`/Game/Models/General/Crate/Crate.Destroy` _ascrate)
      (`/Engine/EditorBlueprintResources/StandardMacros.DoOnce` false :!label _label_2
        (:`Completed`
          (`GameplayStatics.SpawnSoundAtLocation` "/Game/Sounds/akuaku_hit.akuaku_hit")
          (goto _label_2 :!via `Reset`))))))

(fn `UserConstructionScript`)