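; Extra-life pickup for the Crash Bandicoot player, collected on touch or automatically after a delay when AutoEat is set.
; A looping timer polls sphere overlap: an attacking player knocks the pickup away in a random upward direction and destroys it without granting a life.
; Otherwise it calls CallLifeUp, interpolates toward an offset from the player's captured position, then calls LifeUp and destroys itself.
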(event `self.ReceiveBeginPlay`
  (`KismetSystemLibrary.K2_SetTimerDelegate` (delegate `CheckEatStatus`) 0.1 true)
  (`KismetSystemLibrary.Delay` 0.05)
  (`KismetSystemLibrary.Delay` (`self.delay`))
  (if (`self.autoEat`)
    (`/Engine/EditorBlueprintResources/StandardMacros.DoOnce` false
      (:`Completed`
        (bind _ascrash_bandicoot_player_bp (cast `/Game/Main/Blueprints/CrashBandicootPlayerBP` (`GameplayStatics.GetPlayerCharacter` 0)))
        (`/Game/Main/Blueprints/CrashBandicootPlayerBP.lifeUp` _ascrash_bandicoot_player_bp)
        (`self.Inıt Move`)))
    (else
      (`KismetSystemLibrary.Delay` 0.5)
      (set `self.canBeEaten?` true))))

(event `ThrowIt!`
  (`GameplayStatics.PlaySoundAtLocation` "/Game/Sounds/enemyhit.enemyhit" :!label _label)
  (`self.RandomizeX`)
  (`self.RandomizeY`)
  (`self.RandomizeZ`)
  (bind _returnvalue (`KismetSystemLibrary.K2_SetTimerDelegate` (delegate `Throw`) 0.01 true))
  (`KismetSystemLibrary.Delay` 0.5)
  (`KismetSystemLibrary.K2_PauseTimerHandle` _returnvalue)
  (`self.K2_DestroyActor`))

(event `CheckEatStatus`
  (bind _ascrash_bandicoot_player_bp (cast `/Game/Main/Blueprints/CrashBandicootPlayerBP` (`GameplayStatics.GetPlayerCharacter` 0)))
  (if (`PrimitiveComponent.IsOverlappingActor` (`self.Sphere`) _ascrash_bandicoot_player_bp)
    (if (`self.canBeEaten?`)
      (bind _ascrash_bandicoot_player_bp_2 (cast `/Game/Main/Blueprints/CrashBandicootPlayerBP` (`GameplayStatics.GetPlayerCharacter` 0)))
      (`/Engine/EditorBlueprintResources/StandardMacros.DoOnce` false
        (:`Completed`
          (if (or (`/Game/Main/Blueprints/CrashBandicootPlayerBP.isAttacking?` _ascrash_bandicoot_player_bp_2) (`/Game/Main/Blueprints/CrashBandicootPlayerBP.isCrouchAttacking?` _ascrash_bandicoot_player_bp_2) (`/Game/Main/Blueprints/CrashBandicootPlayerBP.isBellyFlopping?` _ascrash_bandicoot_player_bp_2))
            (goto _label)
            (else
              (`/Game/Main/Blueprints/CrashBandicootPlayerBP.lifeUp` _ascrash_bandicoot_player_bp_2)
              (`self.Inıt Move`))))))))

(event `Throw`
  (bind _cube (`self.Cube`))
  (bind (_relativelocation_x _relativelocation_y _relativelocation_z) (`KismetMathLibrary.BreakVector` (`SceneComponent.RelativeLocation` _cube)))
  (`SceneComponent.K2_SetRelativeLocation` _cube (`KismetMathLibrary.MakeVector` (+ _relativelocation_x (`self.randX`)) (+ _relativelocation_y (`self.randY`)) (+ _relativelocation_z (`self.randZ`))) false false))

(event `Inıt Move`
  (bind _ascrash_bandicoot_player_bp (cast `/Game/Main/Blueprints/CrashBandicootPlayerBP` (`GameplayStatics.GetPlayerCharacter` 0)))
  (set `self.vTarget` (+ (`SceneComponent.K2_GetComponentLocation` (`Character.Mesh` _ascrash_bandicoot_player_bp)) (280.0 0.0 280.0)))
  (bind _returnvalue (`KismetSystemLibrary.K2_SetTimerDelegate` (delegate `Move`) 0.01 true))
  (set `self.MOVE_PAUSE` _returnvalue))

(event `Move`
  (bind _returnvalue (`self.K2_GetActorLocation`))
  (bind _vtarget (`self.vTarget`))
  (`self.K2_SetActorLocation` (`KismetMathLibrary.VInterpTo` _returnvalue _vtarget 0.01 (`KismetMathLibrary.RandomFloatInRange` 3.0 5.0)))
  (if (== _returnvalue _vtarget :`ErrorTolerance` 40.0)
    (bind _ascrash_bandicoot_player_bp (cast `/Game/Main/Blueprints/CrashBandicootPlayerBP` (`GameplayStatics.GetPlayerCharacter` 0)))
    (`/Game/Main/Blueprints/CrashBandicootPlayerBP.Life Up` _ascrash_bandicoot_player_bp)
    (`KismetSystemLibrary.K2_PauseTimerHandle` (`self.MOVE_PAUSE`))
    (`self.K2_DestroyActor`)))

(fn `RandomizeX`
  (bind _returnvalue (`KismetMathLibrary.RandomIntegerInRange` 5 10))
  (if (== (`KismetMathLibrary.RandomIntegerInRange` 0 1) 1)
    (bind _result (`/Engine/EditorBlueprintResources/StandardMacros.NegateInt` _returnvalue)
      (:`  `
        (set `self.randX` (`KismetMathLibrary.Conv_IntToDouble` _result))))
    (else
      (set `self.randX` (`KismetMathLibrary.Conv_IntToDouble` _returnvalue)))))

(fn `RandomizeY`
  (bind _returnvalue (`KismetMathLibrary.RandomIntegerInRange` 5 10))
  (if (== (`KismetMathLibrary.RandomIntegerInRange` 0 1) 1)
    (bind _result (`/Engine/EditorBlueprintResources/StandardMacros.NegateInt` _returnvalue)
      (:`  `
        (set `self.randY` (`KismetMathLibrary.Conv_IntToDouble` _result))))
    (else
      (set `self.randY` (`KismetMathLibrary.Conv_IntToDouble` _returnvalue)))))

(fn `RandomizeZ`
  (bind _returnvalue (`KismetMathLibrary.RandomIntegerInRange` 5 10))
  (if (== (`KismetMathLibrary.RandomIntegerInRange` 0) 1)
    (bind _result (`/Engine/EditorBlueprintResources/StandardMacros.NegateInt` _returnvalue)
      (:`  `
        (set `self.randZ` (`KismetMathLibrary.Conv_IntToDouble` _result))))
    (else
      (set `self.randZ` (`KismetMathLibrary.Conv_IntToDouble` _returnvalue)))))

(fn `UserConstructionScript`)