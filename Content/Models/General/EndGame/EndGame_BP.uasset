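; EndGame_BP is the end-of-game warp that sucks the Crash Bandicoot player away and shows the credits.
; Entering Sphere1 fires once, disabling input and gravity, then lifts the player and, after a delay, launches them away with animations, warp sound and credits widget.
; A fast looping timer fakes warp stretching by narrowing the mesh in X/Y at a fixed tall Z scale.
; Reaching the Box stops movement and pauses that timer.
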(event `CustomEvent_0`
  (bind _ascrash_bandicoot_player_bp (cast `/Game/Main/Blueprints/CrashBandicootPlayerBP` (`GameplayStatics.GetPlayerCharacter` 0)))
  (bind _mesh (`Character.Mesh` _ascrash_bandicoot_player_bp))
  (bind (_returnvalue_x _returnvalue_y) (`KismetMathLibrary.BreakVector` (`SceneComponent.K2_GetComponentScale` _mesh)))
  (`SceneComponent.SetWorldScale3D` _mesh (`KismetMathLibrary.MakeVector` (- _returnvalue_x 0.2) (- _returnvalue_y 0.2) 6.3)))

(event `self.Sphere1.OnComponentBeginOverlap`
  (params (OverlappedComponent :type "PrimitiveComponent Object Reference") (OtherActor :type "Actor Object Reference") (OtherComp :type "PrimitiveComponent Object Reference") (OtherBodyIndex :type Integer) (bFromSweep :type Boolean) (SweepResult :type "HitResult Structure (by ref)"))
  (bind _ascrash_bandicoot_player_bp (cast `/Game/Main/Blueprints/CrashBandicootPlayerBP` OtherActor))
  (`/Engine/EditorBlueprintResources/StandardMacros.DoOnce` false
    (:`Completed`
      (`self.DisableInput` _ascrash_bandicoot_player_bp null)
      (bind _charactermovement (`Character.CharacterMovement` _ascrash_bandicoot_player_bp))
      (set `CharacterMovementComponent.GravityScale` 0.0 _charactermovement)
      (`MovementComponent.StopMovementImmediately` _charactermovement)
      (`SkeletalMeshComponent.PlayAnimation` (`Character.Mesh` _ascrash_bandicoot_player_bp) "/Game/Main/Animations/falling.falling" false)
      (`Character.LaunchCharacter` _ascrash_bandicoot_player_bp (0.0 50.0 100.0) false false)
      (`KismetSystemLibrary.Delay` 1.0)
      (`Character.LaunchCharacter` _ascrash_bandicoot_player_bp (0.0 -800.0 -300.0) false false)
      (bind _returnvalue (`KismetSystemLibrary.K2_SetTimerDelegate` (delegate `CustomEvent_0`) 0.01 true))
      (`SkeletalMeshComponent.PlayAnimation` (`Character.Mesh` _ascrash_bandicoot_player_bp) "/Game/Main/Animations/flying.flying" false)
      (`GameplayStatics.SpawnSoundAtLocation` "/Game/Sounds/warpEffect.warpEffect")
      (bind _returnvalue_2 (`|CreateWidget` "/Game/UI/Credits.Credits_C" (`GameplayStatics.GetPlayerController` 0)))
      (`UserWidget.AddToViewport` _returnvalue_2 1))))

(event `self.Box.OnComponentBeginOverlap`
  (params (OverlappedComponent :type "PrimitiveComponent Object Reference") (OtherActor :type "Actor Object Reference") (OtherComp :type "PrimitiveComponent Object Reference") (OtherBodyIndex :type Integer) (bFromSweep :type Boolean) (SweepResult :type "HitResult Structure (by ref)"))
  (bind _ascrash_bandicoot_player_bp (cast `/Game/Main/Blueprints/CrashBandicootPlayerBP` OtherActor))
  (`MovementComponent.StopMovementImmediately` (`Character.CharacterMovement` _ascrash_bandicoot_player_bp))
  (`KismetSystemLibrary.K2_PauseTimerHandle` (stale `self.Sphere1.OnComponentBeginOverlap` _returnvalue)))

(fn `UserConstructionScript`)