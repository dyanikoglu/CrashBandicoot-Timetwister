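; End-of-level crate counter that shows destroyed versus total crates on a spinning display and rewards a full clear with a white gem.
; Looping timers rotate the skeletal mesh and refresh the text from GameInitRef, polling player distance.
; When the player is near, it triggers the end-level matinee and lightning, also spawning the pickable gem and destroying itself if all crates are broken.
; GetIcon maps digits to materials but is uncalled here.
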(event `self.ReceiveBeginPlay`
  (`KismetSystemLibrary.K2_SetTimerDelegate` (delegate `Rotate`) 0.01 true)
  (`KismetSystemLibrary.Delay` 1.0)
  (set `self.totalCrates` (`/Game/Main/Blueprints/GameInitializer_BP.totalCrates` (`self.gameInitRef`)))
  (`KismetSystemLibrary.K2_SetTimerDelegate` (delegate `CheckCrateCount`) 0.5 true))

(event `Rotate`
  (bind _skeletalmesh (`self.SkeletalMesh`))
  (bind _returnvalue (`SceneComponent.K2_GetComponentRotation` _skeletalmesh))
  (`SceneComponent.K2_SetWorldRotation` _skeletalmesh (`KismetMathLibrary.RInterpTo` _returnvalue (`KismetMathLibrary.MakeRotator` (.roll _returnvalue) (.pitch _returnvalue) (+ (.yaw _returnvalue) 1.0)) 1.0 8.0) false false))

(event `CheckCrateCount`
  (bind _endlevelbpref (`self.endLevelBPRef`))
  (bind _endlevelbpref_2 (`self.endLevelBPRef`))
  (`TextRenderComponent.K2_SetText` (`self.TextRender`) (`KismetTextLibrary.Conv_StringToText` (`KismetStringLibrary.Concat_StrStr` (`KismetStringLibrary.Conv_IntToString` (`/Game/Main/Blueprints/GameInitializer_BP.destroyedCrates` (`self.gameInitRef`))) "/" (`KismetStringLibrary.Conv_IntToString` (`self.totalCrates`)))))
  (if (< (`self.GetDistanceTo` (`GameplayStatics.GetPlayerCharacter` 0)) 750.0)
    (if (== (`/Game/Main/Blueprints/GameInitializer_BP.destroyedCrates` (`self.gameInitRef`)) (`self.totalCrates`))
      (bind _returnvalue (`|SpawnActorFromClass` "/Game/Models/General/Crystal/White/WhiteGem_BP.WhiteGem_BP_C" (`KismetMathLibrary.MakeTransform` (- (`self.K2_GetActorLocation`) (0.0 0.0 25.0)) (struct :`Roll` 90.0) (0.8 0.8 0.8)) "Undefined" "OverrideRootScale"))
      (`/Game/Models/General/Crystal/White/WhiteGem_BP.Make Pickable` _returnvalue)
      (`MatineeActor.Play` (`self.endLevelMatinee`))
      (`SceneComponent.SetVisibility` (`/Game/Models/General/EndGame/EndGame_BP.Lightning` _endlevelbpref_2) true false)
      (`ActorComponent.Activate` (`/Game/Models/General/EndGame/EndGame_BP.Lightning_Effect` _endlevelbpref_2) false)
      (`self.K2_DestroyActor`)
      (else
        (`MatineeActor.Play` (`self.endLevelMatinee`))
        (`SceneComponent.SetVisibility` (`/Game/Models/General/EndGame/EndGame_BP.Lightning` _endlevelbpref) true false)
        (`ActorComponent.Activate` (`/Game/Models/General/EndGame/EndGame_BP.Lightning_Effect` _endlevelbpref) false)))))

(fn `getIcon`
  (params (`Num In` :type Integer))
  (returns (`Num Out` :type "Material Object Reference"))
  (switch `int` `Num In`
    (:`Default`
      _)
    (:`0`
      _)
    (:`1`
      (return "/Game/UI/Wumpa/Count/1_Mat.1_Mat"))
    (:`2`
      (return "/Game/UI/Wumpa/Count/2_Mat.2_Mat"))
    (:`3`
      (return "/Game/UI/Wumpa/Count/3_Mat.3_Mat"))
    (:`4`
      (return "/Game/UI/Wumpa/Count/4_Mat.4_Mat"))
    (:`5`
      (return "/Game/UI/Wumpa/Count/5_Mat.5_Mat"))
    (:`6`
      (return "/Game/UI/Wumpa/Count/6_Mat.6_Mat"))
    (:`7`
      (return "/Game/UI/Wumpa/Count/7_Mat.7_Mat"))
    (:`8`
      (return "/Game/UI/Wumpa/Count/8_Mat.8_Mat"))
    (:`9`
      (return "/Game/UI/Wumpa/Count/9_Mat.9_Mat")))
  (return "/Game/UI/Wumpa/Count/0_Mat.0_Mat"))

(fn `UserConstructionScript`)