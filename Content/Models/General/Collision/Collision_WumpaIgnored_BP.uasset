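; Trigger volume that pauses a timer on its linked Door_BP when the Crash Bandicoot player overlaps it.
; The construction script links the door by scanning all Door_BP actors for the first whose first tag matches its own and storing it as DoorRef.
; Overlap on the Pass component casts to the player Blueprint, then pauses that door's PAUSE timer handle.
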(event `self.Pass.OnComponentBeginOverlap`
  (params (OverlappedComponent :type "PrimitiveComponent Object Reference") (OtherActor :type "Actor Object Reference") (OtherComp :type "PrimitiveComponent Object Reference") (OtherBodyIndex :type Integer) (bFromSweep :type Boolean) (SweepResult :type "HitResult Structure (by ref)"))
  (cast `/Game/Main/Blueprints/CrashBandicootPlayerBP` OtherActor)
  (`KismetSystemLibrary.K2_PauseTimerHandle` (`/Game/Models/Misc/TombWader/Door/Door_BP.PAUSE` (`self.Door_Ref`))))

(fn `UserConstructionScript`
  (bind _outactors (`GameplayStatics.GetAllActorsOfClass` "/Game/Models/Misc/TombWader/Door/Door_BP.Door_BP_C"))
  (for _array_element _outactors
    (if (== (`KismetArrayLibrary.Array_Get` (`Actor.Tags` _array_element)) (`KismetArrayLibrary.Array_Get` (`self.Tags`)))
      (bind _asdoor_bp (cast `/Game/Models/Misc/TombWader/Door/Door_BP` _array_element))
      (set `self.Door_Ref` _asdoor_bp)
      (break))))