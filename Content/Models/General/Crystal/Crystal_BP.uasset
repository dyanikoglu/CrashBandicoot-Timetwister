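; Crystal pickup that reacts once when the Crash Bandicoot player overlaps its capsule.
; It hides the crystal, plays its sound at the world origin and deactivates the glow.
; One point light flashes bright briefly before both lights drop to zero intensity.
; The actor is not destroyed, and the Blueprint records no collection count or player state.
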(event `self.Capsule.OnComponentBeginOverlap`
  (params (OverlappedComponent :type "PrimitiveComponent Object Reference") (OtherActor :type "Actor Object Reference") (OtherComp :type "PrimitiveComponent Object Reference") (OtherBodyIndex :type Integer) (bFromSweep :type Boolean) (SweepResult :type "HitResult Structure (by ref)"))
  (bind _pointlight (`self.PointLight`))
  (cast `/Game/Main/Blueprints/CrashBandicootPlayerBP` OtherActor)
  (`/Engine/EditorBlueprintResources/StandardMacros.DoOnce` false
    (:`Completed`
      (`SceneComponent.SetHiddenInGame` (`self.Crystal`) true false)
      (`GameplayStatics.PlaySoundAtLocation` "/Game/Sounds/crystal.crystal")
      (`ActorComponent.Deactivate` (`self.glow`))
      (`LightComponent.SetIntensity` _pointlight 10000.0)
      (`KismetSystemLibrary.Delay` 0.3)
      (`LightComponent.SetIntensity` _pointlight 0.0)
      (`LightComponent.SetIntensity` (`self.PointLight1`) 0.0))))

(fn `UserConstructionScript`)