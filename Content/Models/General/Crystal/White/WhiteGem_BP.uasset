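; WhiteGem_BP is a white gem pickup that the Crash Bandicoot player collects once it has been made pickable.
; MakePickable sets the Pickable flag, shows the gem mesh, and plays a crystal sound and dash particle effect.
; When Pickable, overlap by CrashBandicootPlayerBP plays the sound, spawns loot particles and destroys the actor, without recording the collection.
; Both sounds play at the world origin rather than at the gem.
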(event `Make Pickable`
  (set `self.pickable` true)
  (`SceneComponent.SetVisibility` (`self.Gem`) true false)
  (`GameplayStatics.PlaySoundAtLocation` "/Game/Sounds/crystal.crystal")
  (`GameplayStatics.SpawnEmitterAtLocation` "/Game/Effects/Effects/FX_Monsters/FX_Monster_Elemental/ICE/P_JumpAndDive_Dash.P_JumpAndDive_Dash" (+ (`SceneComponent.K2_GetComponentLocation` (`self.DefaultSceneRoot`)) (-78.0 0.0 30.0))))

(event `self.Gem.OnComponentBeginOverlap`
  (params (OverlappedComponent :type "PrimitiveComponent Object Reference") (OtherActor :type "Actor Object Reference") (OtherComp :type "PrimitiveComponent Object Reference") (OtherBodyIndex :type Integer) (bFromSweep :type Boolean) (SweepResult :type "HitResult Structure (by ref)"))
  (if (`self.pickable`)
    (cast `/Game/Main/Blueprints/CrashBandicootPlayerBP` OtherActor)
    (`GameplayStatics.SpawnSoundAtLocation` "/Game/Sounds/crystal.crystal")
    (`GameplayStatics.SpawnEmitterAtLocation` "/Game/Effects/Effects/FX_Treasure/Loot/P_Loot_Pickup.P_Loot_Pickup" (+ (`SceneComponent.K2_GetComponentLocation` (`self.DefaultSceneRoot`)) (0.0 0.0 0.0)))
    (`self.K2_DestroyActor`)))

(fn `UserConstructionScript`)