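; Phara enemy character from the TombWader set that chases Crash and guards itself with a movable shield.
; A looping distance check starts or pauses, through paired DoOnce gates, a faster timer that moves it toward nearby Crash.
; That timer also flips the shield to an upside pose when Crash is well above.
; Body hits kill the attacking player's target or else Crash, while attacked shield hits only pulse an impact flag and sound.
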(event `Check Crash`
  (bind (_returnvalue_x _returnvalue_y _returnvalue_z) (`KismetMathLibrary.BreakVector` (`SceneComponent.K2_GetComponentLocation` (`self.Mesh`))))
  (bind _ascrash_bandicoot_player_bp (cast `/Game/Main/Blueprints/CrashBandicootPlayerBP` (`GameplayStatics.GetPlayerCharacter` 0)))
  (`AIBlueprintHelperLibrary.SimpleMoveToActor` (`self.GetController`) _ascrash_bandicoot_player_bp)
  (bind _mesh (`Character.Mesh` _ascrash_bandicoot_player_bp))
  (`/Engine/EditorBlueprintResources/StandardMacros.IsValid` _mesh
    (:`Is Valid`
      (bind (_returnvalue_x_2 _returnvalue_y_2 _returnvalue_z_2) (`KismetMathLibrary.BreakVector` (`SceneComponent.K2_GetComponentLocation` _mesh)))
      (if (> (- _returnvalue_z_2 _returnvalue_z) 150.0)
        (set `self.isCrashUpside?` true)
        (`SceneComponent.K2_SetRelativeLocationAndRotation` (`self.Shield`) (`self.upsideShieldLoc`) (`self.upsideShieldRot`) false true)
        (else
          (set `self.isCrashUpside?` false)
          (`SceneComponent.K2_SetRelativeLocationAndRotation` (`self.Shield`) (`self.normalShieldLoc`) (`self.normalShieldRot`) false true))))))

(event `self.ReceiveBeginPlay`
  (`KismetSystemLibrary.K2_SetTimerDelegate` (delegate `CheckDistance`) 0.1 true))

(event `CheckDistance`
  (bind _returnvalue (`GameplayStatics.GetPlayerCharacter` 0))
  (`/Engine/EditorBlueprintResources/StandardMacros.IsValid` _returnvalue
    (:`Is Valid`
      (if (`self.isDead?`)
        _
        (elif (< (`KismetMathLibrary.VSize` (- (`self.K2_GetActorLocation` _returnvalue) (`self.K2_GetActorLocation`))) 650.0)
          (set `self.isCrashNear?` true)
          (`/Engine/EditorBlueprintResources/StandardMacros.DoOnce` false :!label _label
            (:`Completed`
              (bind _returnvalue_2 (`KismetSystemLibrary.K2_SetTimerDelegate` (delegate `Check Crash`) 0.05 true))
              (set `self.PAUSE` _returnvalue_2)
              (goto _label_2 :!via `Reset`)))
          (else
            _)))
      (set `self.isCrashNear?` false)
      (`/Engine/EditorBlueprintResources/StandardMacros.DoOnce` false :!label _label_2
        (:`Completed`
          (`KismetSystemLibrary.K2_PauseTimerHandle` (`self.PAUSE`))
          (goto _label :!via `Reset`))))))

(event `self.CapsuleComponent.OnComponentHit`
  (params (HitComponent :type "PrimitiveComponent Object Reference") (OtherActor :type "Actor Object Reference") (OtherComp :type "PrimitiveComponent Object Reference") (NormalImpulse :type "Vector Structure") (Hit :type "HitResult Structure (by ref)"))
  (bind _ascrash_bandicoot_player_bp (cast `/Game/Main/Blueprints/CrashBandicootPlayerBP` OtherActor))
  (if (or (`/Game/Main/Blueprints/CrashBandicootPlayerBP.isAttacking?` _ascrash_bandicoot_player_bp) (`/Game/Main/Blueprints/CrashBandicootPlayerBP.isCrouchAttacking?` _ascrash_bandicoot_player_bp))
    (`self.Throw Death`)
    (else
      (`/Game/Main/Blueprints/CrashBandicootPlayerBP.Death` _ascrash_bandicoot_player_bp 0))))

(event `self.Shield.OnComponentHit`
  (params (HitComponent :type "PrimitiveComponent Object Reference") (OtherActor :type "Actor Object Reference") (OtherComp :type "PrimitiveComponent Object Reference") (NormalImpulse :type "Vector Structure") (Hit :type "HitResult Structure (by ref)"))
  (bind _ascrash_bandicoot_player_bp (cast `/Game/Main/Blueprints/CrashBandicootPlayerBP` OtherActor))
  (if (`/Game/Main/Blueprints/CrashBandicootPlayerBP.isAttacking?` _ascrash_bandicoot_player_bp)
    (`/Engine/EditorBlueprintResources/StandardMacros.DoOnce` false :!label _label_3
      (:`Completed`
        (set `self.impact!` true)
        (`GameplayStatics.SpawnSoundAttached` "/Game/Sounds/shield.shield" (`self.Mesh`) "None" (0.0 0.0 0.0) (struct) "KeepRelativeOffset" false 1.0 1.0 0.0 null null)
        (`KismetSystemLibrary.Delay` 0.1)
        (set `self.impact!` false)
        (goto _label_3 :!via `Reset`)))))

(fn `UserConstructionScript`)