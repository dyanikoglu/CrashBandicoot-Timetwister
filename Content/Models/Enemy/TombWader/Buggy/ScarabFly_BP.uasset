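; Scarab enemy Blueprint that kills Crash on body contact unless he is attacking, belly-flopping or crouch-attacking, which triggers ThrowDeath instead.
; A timed BeginPlay loop alternates the skeletal mesh and looping animation between Scarab_Move and Bug_fixed, without affecting the collision logic.
; The JumpOver overlap handles a falling player: attacks trigger ThrowDeath, while a plain landing calls StandartDeath and bounces Crash via LaunchCrash.
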(event `self.ReceiveBeginPlay`
  (`KismetSystemLibrary.Delay` 4.0 :!label _label)
  (`SkinnedMeshComponent.SetSkinnedAssetAndUpdate` (`self.Mesh`) "/Game/Models/Enemy/TombWader/Buggy/Scarab_Move.Scarab_Move" true)
  (`SkeletalMeshComponent.PlayAnimation` (`self.Mesh`) "/Game/Models/Enemy/TombWader/Buggy/Scarab_Move_Anim.Scarab_Move_Anim" true)
  (`KismetSystemLibrary.Delay` 4.0)
  (`SkinnedMeshComponent.SetSkinnedAssetAndUpdate` (`self.Mesh`) "/Game/Models/Enemy/TombWader/Buggy/bug_fixed.bug_fixed" true)
  (`SkeletalMeshComponent.PlayAnimation` (`self.Mesh`) "/Game/Models/Enemy/TombWader/Buggy/bug_fixed_Anim.bug_fixed_Anim" true)
  (`KismetSystemLibrary.Delay` 2.0)
  (goto _label))

(event `self.Capsule.OnComponentBeginOverlap`
  (params (OverlappedComponent :type "PrimitiveComponent Object Reference") (OtherActor :type "Actor Object Reference") (OtherComp :type "PrimitiveComponent Object Reference") (OtherBodyIndex :type Integer) (bFromSweep :type Boolean) (SweepResult :type "HitResult Structure (by ref)"))
  (if (not (`self.isDead?`))
    (bind _ascrash_bandicoot_player_bp (cast `/Game/Main/Blueprints/CrashBandicootPlayerBP` OtherActor))
    (if (or (`/Game/Main/Blueprints/CrashBandicootPlayerBP.isAttacking?` _ascrash_bandicoot_player_bp) (`/Game/Main/Blueprints/CrashBandicootPlayerBP.isBellyFlopping?` _ascrash_bandicoot_player_bp) (`/Game/Main/Blueprints/CrashBandicootPlayerBP.isCrouchAttacking?` _ascrash_bandicoot_player_bp))
      (`self.Throw Death` :!label _label_2)
      (else
        (`/Game/Main/Blueprints/CrashBandicootPlayerBP.Death` _ascrash_bandicoot_player_bp 0)))))

(event `self.jumpOver.OnComponentBeginOverlap`
  (params (OverlappedComponent :type "PrimitiveComponent Object Reference") (OtherActor :type "Actor Object Reference") (OtherComp :type "PrimitiveComponent Object Reference") (OtherBodyIndex :type Integer) (bFromSweep :type Boolean) (SweepResult :type "HitResult Structure (by ref)"))
  (bind _ascrash_bandicoot_player_bp (cast `/Game/Main/Blueprints/CrashBandicootPlayerBP` OtherActor))
  (if (`NavMovementComponent.IsFalling` (`Character.CharacterMovement` _ascrash_bandicoot_player_bp))
    (if (or (`/Game/Main/Blueprints/CrashBandicootPlayerBP.isAttacking?` _ascrash_bandicoot_player_bp) (`/Game/Main/Blueprints/CrashBandicootPlayerBP.isBellyFlopping?` _ascrash_bandicoot_player_bp) (`/Game/Main/Blueprints/CrashBandicootPlayerBP.isCrouchAttacking?` _ascrash_bandicoot_player_bp))
      (goto _label_2)
      (else
        (`self.Standart Death`)
        (`/Game/Main/Blueprints/CrashBandicootPlayerBP.LaunchCrash` _ascrash_bandicoot_player_bp)))))

(fn `UserConstructionScript`)