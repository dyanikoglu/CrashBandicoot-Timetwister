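; Mummy enemy for the TombWader level that hops after Crash while he is nearby and kills him on contact.
; A looping distance check starts or pauses a fast movement timer that repeatedly jumps and moves toward the player, gated by paired DoOnce nodes.
; The JumpOver trigger destroys the mummy if Crash is attacking, otherwise kills him, as does the Death trigger.
; Hitting a blocking volume plays a sound and animation.
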(event `self.ReceiveBeginPlay`
  (`KismetSystemLibrary.K2_SetTimerDelegate` (delegate `CheckDistance`) 0.1 true))

(event `CheckDistance`
  (bind _returnvalue (`GameplayStatics.GetPlayerCharacter` 0))
  (`/Engine/EditorBlueprintResources/StandardMacros.IsValid` _returnvalue
    (:`Is Valid`
      (if (`self.isDead?`)
        _
        (elif (< (`KismetMathLibrary.VSize` (- (`self.K2_GetActorLocation` _returnvalue) (`self.K2_GetActorLocation`))) 1000.0)
          (set `self.isCrashNear?` true)
          (`/Engine/EditorBlueprintResources/StandardMacros.DoOnce` false :!label _label
            (:`Completed`
              (bind _returnvalue_2 (`KismetSystemLibrary.K2_SetTimerDelegate` (delegate `Update Move`) 0.005 true))
              (set `self.PAUSE` _returnvalue_2)
              (goto _label_2 :!via `Reset`)))
          (else
            _)))
      (set `self.isCrashNear?` false)
      (`/Engine/EditorBlueprintResources/StandardMacros.DoOnce` false :!label _label_2
        (:`Completed`
          (`KismetSystemLibrary.K2_PauseTimerHandle` (`self.PAUSE`))
          (goto _label :!via `Reset`))))))

(event `Update Move`
  (bind (_returnvalue_x _returnvalue_y _returnvalue_z) (`KismetMathLibrary.BreakVector` (`SceneComponent.K2_GetComponentLocation` (`self.CapsuleComponent`))))
  (bind _ascrash_bandicoot_player_bp (cast `/Game/Main/Blueprints/CrashBandicootPlayerBP` (`GameplayStatics.GetPlayerCharacter` 0)))
  (if (and (not (`/Game/Main/Blueprints/CrashBandicootPlayerBP.isDead?` _ascrash_bandicoot_player_bp)) (not (`self.isDead?`)))
    (`self.Jump`)
    (bind (_returnvalue_x_2 _returnvalue_y_2) (`KismetMathLibrary.BreakVector` (`SceneComponent.K2_GetComponentLocation` (`Character.Mesh` _ascrash_bandicoot_player_bp))))
    (`AIBlueprintHelperLibrary.SimpleMoveToLocation` (`self.GetController`) (`KismetMathLibrary.MakeVector` _returnvalue_x_2 _returnvalue_y_2 _returnvalue_z))))

(event `self.CapsuleComponent.OnComponentHit`
  (params (HitComponent :type "PrimitiveComponent Object Reference") (OtherActor :type "Actor Object Reference") (OtherComp :type "PrimitiveComponent Object Reference") (NormalImpulse :type "Vector Structure") (Hit :type "HitResult Structure (by ref)"))
  (bind _mesh (`self.Mesh`))
  (if (not (`self.isDead?`))
    (cast `BlockingVolume` OtherActor)
    (`GameplayStatics.SpawnSoundAttached` "/Game/Sounds/mummy.mummy" _mesh "None" (0.0 0.0 0.0) (struct) "KeepRelativeOffset" false 1.0 1.0 0.0 null null)
    (`SkeletalMeshComponent.PlayAnimation` _mesh "/Game/Models/Enemy/TombWader/Mummy/TEST2_Anim.TEST2_Anim" false)))

(event `self.JumpOver.OnComponentBeginOverlap`
  (params (OverlappedComponent :type "PrimitiveComponent Object Reference") (OtherActor :type "Actor Object Reference") (OtherComp :type "PrimitiveComponent Object Reference") (OtherBodyIndex :type Integer) (bFromSweep :type Boolean) (SweepResult :type "HitResult Structure (by ref)"))
  (bind _ascrash_bandicoot_player_bp (cast `/Game/Main/Blueprints/CrashBandicootPlayerBP` OtherActor))
  (if (and (`/Game/Main/Blueprints/CrashBandicootPlayerBP.isAttacking?` _ascrash_bandicoot_player_bp) (not (`/Game/Main/Blueprints/CrashBandicootPlayerBP.isDead?` _ascrash_bandicoot_player_bp)))
    (`/Engine/EditorBlueprintResources/StandardMacros.DoOnce` false
      (:`Completed`
        (set `self.isDead?` true)
        (`GameplayStatics.SpawnEmitterAtLocation` "/Game/Effects/Effects/FX_Monsters/FX_Monster_FrostGiant/ICE/P_FootSteps_Wa_2.P_FootSteps_Wa_2" (`SceneComponent.K2_GetComponentLocation` (`self.CapsuleComponent`)))
        (`self.K2_DestroyActor`)))
    (else
      (bind _ascrash_bandicoot_player_bp_2 (cast `/Game/Main/Blueprints/CrashBandicootPlayerBP` OtherActor))
      (`/Engine/EditorBlueprintResources/StandardMacros.DoOnce` false
        (:`Completed`
          (`Controller.StopMovement` (`self.GetController`))
          (`/Game/Main/Blueprints/CrashBandicootPlayerBP.Death` _ascrash_bandicoot_player_bp_2 3))))))

(event `self.Death.OnComponentBeginOverlap`
  (params (OverlappedComponent :type "PrimitiveComponent Object Reference") (OtherActor :type "Actor Object Reference") (OtherComp :type "PrimitiveComponent Object Reference") (OtherBodyIndex :type Integer) (bFromSweep :type Boolean) (SweepResult :type "HitResult Structure (by ref)"))
  (if (not (`self.isDead?`))
    (bind _ascrash_bandicoot_player_bp (cast `/Game/Main/Blueprints/CrashBandicootPlayerBP` OtherActor))
    (`/Engine/EditorBlueprintResources/StandardMacros.DoOnce` false
      (:`Completed`
        (`Controller.StopMovement` (`self.GetController`))
        (`/Game/Main/Blueprints/CrashBandicootPlayerBP.Death` _ascrash_bandicoot_player_bp 3)))))

(fn `UserConstructionScript`)