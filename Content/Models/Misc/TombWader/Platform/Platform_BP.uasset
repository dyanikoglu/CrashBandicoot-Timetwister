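; Tilting wooden platform that rolls according to where the player stands on it and eases back to its base rotation otherwise.
; A looping timer checks player overlap with a sphere, then interpolates the mesh's roll toward a value taken from the world Y offset between platform and player mesh.
; A quadrant-sorting Mux macro is defined but unused in these graphs.
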(event `self.ReceiveBeginPlay`
  (`KismetSystemLibrary.K2_SetTimerDelegate` (delegate `CheckCol`) 0.01 true))

(event `CheckCol`
  (bind _wood_platform_lpuv (`self.Wood_Platform_LPUV`))
  (bind _wood_platform_lpuv_2 (`self.Wood_Platform_LPUV`))
  (bind _relativerotation (`SceneComponent.RelativeRotation` _wood_platform_lpuv))
  (bind (_returnvalue_x _returnvalue_y) (`KismetMathLibrary.BreakVector` (- (`SceneComponent.K2_GetComponentLocation` (`self.Wood_Platform_LPUV`)) (`SceneComponent.K2_GetComponentLocation` (`Character.Mesh` (`GameplayStatics.GetPlayerCharacter` 0))))))
  (if (`PrimitiveComponent.IsOverlappingActor` (`self.Sphere`) (`GameplayStatics.GetPlayerCharacter` 0))
    (`SceneComponent.K2_SetRelativeRotation` _wood_platform_lpuv (`KismetMathLibrary.RInterpTo` _relativerotation (`KismetMathLibrary.MakeRotator` (* _returnvalue_y -1.0) (.pitch _relativerotation) (.yaw _relativerotation)) (`GameplayStatics.GetWorldDeltaSeconds`) 1.0) false false)
    (else
      (`SceneComponent.K2_SetRelativeRotation` _wood_platform_lpuv_2 (`KismetMathLibrary.RInterpTo` (`SceneComponent.RelativeRotation` _wood_platform_lpuv_2) (`self.baseRotation`) (`GameplayStatics.GetWorldDeltaSeconds`) 1.0) false false))))

(fn `UserConstructionScript`)