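; Tomb Wader door Blueprint that kills Crash Bandicoot when he overlaps its Death component while the door is not open.
; Check starts a looping timer that counts while Crash stays in range, then pauses, plays MatineeRef and clears IsOpen once he leaves or time runs out.
; The death overlap fires once and also plays OpenRef.
; The construction script caches a Collision_WumpaIgnored_BP actor by matching first tags.
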(event `Check`
  (bind _returnvalue (`KismetSystemLibrary.K2_SetTimerDelegate` (delegate `isCrashNear?`) 1.0 true))
  (set `self.PAUSE` _returnvalue))

(event `isCrashNear?`
  (if (and (< (`KismetMathLibrary.Abs` (`KismetMathLibrary.VSize` (- (`SceneComponent.K2_GetComponentLocation` (`self.Door`)) (`SceneComponent.K2_GetComponentLocation` (`Character.Mesh` (`GameplayStatics.GetPlayerCharacter` 0)))))) (`self.Range`)) (< (`self.timeOut`) 4.0))
    (`/Engine/EditorBlueprintResources/StandardMacros.IncrementFloat` (`self.timeOut`))
    (else
      (`KismetSystemLibrary.K2_PauseTimerHandle` (`self.PAUSE`))
      (`MatineeActor.Play` (`self.Matinee_Ref`))
      (set `self.timeOut` 0.0)
      (set `self.isOpen?` false))))

(event `self.Death.OnComponentBeginOverlap`
  (params (OverlappedComponent :type "PrimitiveComponent Object Reference") (OtherActor :type "Actor Object Reference") (OtherComp :type "PrimitiveComponent Object Reference") (OtherBodyIndex :type Integer) (bFromSweep :type Boolean) (SweepResult :type "HitResult Structure (by ref)"))
  (if (not (`self.isOpen?`))
    (bind _ascrash_bandicoot_player_bp (cast `/Game/Main/Blueprints/CrashBandicootPlayerBP` OtherActor))
    (`/Engine/EditorBlueprintResources/StandardMacros.DoOnce` false
      (:`Completed`
        (`/Game/Main/Blueprints/CrashBandicootPlayerBP.Death` _ascrash_bandicoot_player_bp 2)
        (`MatineeActor.Play` (`self.Open_Ref`))))))

(fn `UserConstructionScript`
  (bind _outactors (`GameplayStatics.GetAllActorsOfClass` "/Game/Models/General/Collision/Collision_WumpaIgnored_BP.Collision_WumpaIgnored_BP_C"))
  (for _array_element _outactors
    (if (== (`|GetArrayItem` (`Actor.Tags` _array_element)) (`|GetArrayItem` (`self.Tags`)))
      (bind _ascollision_wumpa_ignored_bp (cast `/Game/Models/General/Collision/Collision_WumpaIgnored_BP` _array_element))
      (set `self.PassCollision_Ref` _ascollision_wumpa_ignored_bp)
      (break))))