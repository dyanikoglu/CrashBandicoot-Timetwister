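; Wheel_BP is a Tomb Wader wheel that opens a linked door when Crash Bandicoot attacks while overlapping it.
; A looping timer started at BeginPlay polls every tenth of a second for the player's overlap with the Wheel component and their attacking state.
; If the referenced door is still closed, it plays the referenced Matinee, flags the door as open and calls the door's Check.
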(event `self.ReceiveBeginPlay`
  (`KismetSystemLibrary.K2_SetTimerDelegate` (delegate `CustomEvent_0`) 0.1 true))

(event `CustomEvent_0`
  (bind _returnvalue (`GameplayStatics.GetPlayerCharacter` 0))
  (bind _door_ref (`self.Door Ref`))
  (bind _ascrash_bandicoot_player_bp (cast `/Game/Main/Blueprints/CrashBandicootPlayerBP` _returnvalue))
  (if (`PrimitiveComponent.IsOverlappingActor` (`self.Wheel`) _ascrash_bandicoot_player_bp)
    (if (not (`/Game/Models/Misc/TombWader/Door/Door_BP.isOpen?` (`self.Door Ref`)))
      (bind _ascrash_bandicoot_player_bp_2 (cast `/Game/Main/Blueprints/CrashBandicootPlayerBP` _returnvalue))
      (if (`/Game/Main/Blueprints/CrashBandicootPlayerBP.isAttacking?` _ascrash_bandicoot_player_bp_2)
        (`MatineeActor.Play` (`self.Matinee Ref`))
        (set `/Game/Models/Misc/TombWader/Door/Door_BP.isOpen?` true _door_ref)
        (`/Game/Models/Misc/TombWader/Door/Door_BP.Check` _door_ref)))))

(fn `UserConstructionScript`)