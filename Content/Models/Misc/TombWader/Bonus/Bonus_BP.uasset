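; Bonus Blueprint in the TombWader model set that toggles four collision boxes and the Crash Bandicoot player's abilities.
; Enable sets the boxes to BlockAll and turns off the player's jump and attack.
; Disable sets them to OverlapAll and restores both abilities.
; Neither event is triggered within this Blueprint, and both reach the player by casting player character 0.
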(event `Enable`
  (`PrimitiveComponent.SetCollisionProfileName` (`self.Box2`) "BlockAll")
  (`PrimitiveComponent.SetCollisionProfileName` (`self.Box1`) "BlockAll")
  (`PrimitiveComponent.SetCollisionProfileName` (`self.Box`) "BlockAll")
  (`PrimitiveComponent.SetCollisionProfileName` (`self.Box3`) "BlockAll")
  (bind _ascrash_bandicoot_player_bp (cast `/Game/Main/Blueprints/CrashBandicootPlayerBP` (`GameplayStatics.GetPlayerCharacter` 0)))
  (set `/Game/Main/Blueprints/CrashBandicootPlayerBP.canJump?` false _ascrash_bandicoot_player_bp)
  (set `/Game/Main/Blueprints/CrashBandicootPlayerBP.canAttack?` false _ascrash_bandicoot_player_bp))

(event `Disable`
  (`PrimitiveComponent.SetCollisionProfileName` (`self.Box2`) "OverlapAll")
  (`PrimitiveComponent.SetCollisionProfileName` (`self.Box1`) "OverlapAll")
  (`PrimitiveComponent.SetCollisionProfileName` (`self.Box`) "OverlapAll")
  (`PrimitiveComponent.SetCollisionProfileName` (`self.Box3`) "OverlapAll")
  (bind _ascrash_bandicoot_player_bp (cast `/Game/Main/Blueprints/CrashBandicootPlayerBP` (`GameplayStatics.GetPlayerCharacter` 0)))
  (set `/Game/Main/Blueprints/CrashBandicootPlayerBP.canJump?` true _ascrash_bandicoot_player_bp)
  (set `/Game/Main/Blueprints/CrashBandicootPlayerBP.canAttack?` true _ascrash_bandicoot_player_bp))

(fn `UserConstructionScript`)